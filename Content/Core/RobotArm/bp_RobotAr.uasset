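; Robot arm actor that aims at a current product and shows its product Filter as a color.
; The construction script creates a dynamic material on Base and sets ProductColor from the Filter value.
; RotateWithProduct snaps ArmBase yaw and Pivot rotation onto the product, while LookAtNewProduct eases toward it by per-call lerp and reports alignment from a signed yaw delta.
; The event graph is empty, so neither aiming function is called here.
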(event `self.ReceiveTick`
  (params (DeltaSeconds :type "Float (single-precision)")))

(fn `LookAtNewProduct`
  (returns (lookingDone :type Boolean))
  (bind _arm_base (`self.Arm_base`))
  (bind _pivot (`self.pivot`))
  (bind _returnvalue (`SceneComponent.K2_GetComponentRotation` _pivot))
  (bind _returnvalue_2 (`SceneComponent.K2_GetComponentRotation` _arm_base))
  (bind _returnvalue_3 (`KismetMathLibrary.FindLookAtRotation` (`SceneComponent.K2_GetComponentLocation` _arm_base) (`self.K2_GetActorLocation` (`self.currentProduct`))))
  (`SceneComponent.K2_AddWorldRotation` _arm_base (`KismetMathLibrary.MakeRotator` 0.0 0.0 (.yaw (`KismetMathLibrary.NormalizedDeltaRotator` (`KismetMathLibrary.RLerp` _returnvalue_2 _returnvalue_3 0.1) _returnvalue_2))) false false)
  (`SceneComponent.K2_AddWorldRotation` _pivot (`KismetMathLibrary.MakeRotator` (.roll (`KismetMathLibrary.NormalizedDeltaRotator` (`KismetMathLibrary.RLerp` _returnvalue (`KismetMathLibrary.FindLookAtRotation` (`SceneComponent.K2_GetComponentLocation` _pivot) (`self.K2_GetActorLocation` (`self.currentProduct`))) 0.1) _returnvalue)) (.pitch (`KismetMathLibrary.NormalizedDeltaRotator` (`KismetMathLibrary.RLerp` _returnvalue (`KismetMathLibrary.FindLookAtRotation` (`SceneComponent.K2_GetComponentLocation` _pivot) (`self.K2_GetActorLocation` (`self.currentProduct`))) 0.1) _returnvalue))) false false)
  (bind _output_get (set `self.LookingAtNewProduct` (< (.yaw (`KismetMathLibrary.NormalizedDeltaRotator` _returnvalue_3 _returnvalue_2)) 5.0)))
  (return _output_get))

(fn `RotateWithProduct`
  (bind _arm_base (`self.Arm_base`))
  (bind _pivot (`self.pivot`))
  (`SceneComponent.K2_SetWorldRotation` _arm_base (`KismetMathLibrary.MakeRotator` 0.0 0.0 (.yaw (`KismetMathLibrary.FindLookAtRotation` (`SceneComponent.K2_GetComponentLocation` _arm_base) (`self.K2_GetActorLocation` (`self.currentProduct`))))) true false)
  (`SceneComponent.K2_SetWorldRotation` _pivot (`KismetMathLibrary.FindLookAtRotation` (`SceneComponent.K2_GetComponentLocation` _pivot) (`self.K2_GetActorLocation` (`self.currentProduct`))) true false))

(fn `UserConstructionScript`
  (bind _returnvalue (`PrimitiveComponent.CreateDynamicMaterialInstance` (`self.Base`) 0 "/Game/Core/RobotArm/M_RobotArmB.M_RobotArmB" "None"))
  (bind _output_get (set `self.DynColor` _returnvalue))
  (switch `EDestCode` (`self.filter`)
    (:`AA`
      (`MaterialInstanceDynamic.SetVectorParameterValue` _output_get "ProductColor" (`KismetMathLibrary.MakeColor` 1.0)))
    (:`BB`
      (`MaterialInstanceDynamic.SetVectorParameterValue` _output_get "ProductColor" (`KismetMathLibrary.MakeColor` 0.0 0.0 1.0)))
    (:`CC`
      (`MaterialInstanceDynamic.SetVectorParameterValue` _output_get "ProductColor" (struct :`R` 0.054902 :`G` 0.862745 :`B` 0.043137 :`A` 1.0)))
    (:`DD`
      (`MaterialInstanceDynamic.SetVectorParameterValue` _output_get "ProductColor" (`KismetMathLibrary.MakeColor` 1.0 1.0)))
    (:`EE`
      (`MaterialInstanceDynamic.SetVectorParameterValue` _output_get "ProductColor" (`KismetMathLibrary.MakeColor` 1.0 0.0 1.0)))
    (:`FF`
      (`MaterialInstanceDynamic.SetVectorParameterValue` _output_get "ProductColor" (`KismetMathLibrary.MakeColor` 0.0 1.0 1.0)))
    (:`GG`
      (`MaterialInstanceDynamic.SetVectorParameterValue` _output_get "ProductColor" (`KismetMathLibrary.MakeColor` 1.0 0.2 0.2)))
    (:`HH`
      (`MaterialInstanceDynamic.SetVectorParameterValue` _output_get "ProductColor" (`KismetMathLibrary.MakeColor` 1.0 1.0 1.0)))
    (:`None`
      (`MaterialInstanceDynamic.SetVectorParameterValue` _output_get "ProductColor" (`KismetMathLibrary.MakeColor` 0.0)))))