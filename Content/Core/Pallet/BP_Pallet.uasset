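; BP_Pallet is a pallet actor that a jack pawn can carry, with a product count that is full at 24.
; Each tick it rescales its placement HUD widget by distance to the player's pawn, growing as distance increases.
; While Moving, it snaps to the jack's handle with a 90-degree yaw offset.
; ClosestPickupPoint returns the nearer of two sphere locations; product stacking debug code is left disconnected.
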(event `self.ReceiveBeginPlay`
  ;[1 1 1] Init
  (bind _aspallet_placement_hud (cast `/Game/Core/HUD/PalletPlacement_HUD` (`WidgetComponent.GetUserWidgetObject` (`self.Widget`))))
  (set `self.As Pallet Placement HUD` _aspallet_placement_hud)
  (bind _asbp_robotics_fcplayer_controller (cast `/Game/TopDownCPP/Blueprints/BP_RoboticsFCPlayerController` (`GameplayStatics.GetPlayerController` 0)))
  (set `self.Player Con` _asbp_robotics_fcplayer_controller))

(event `self.ReceiveTick`
  (params (DeltaSeconds :type "Float (single-precision)"))
  (`|ExecutionSequence`
    (:`then_0`
      (`self.Resize Widget to Screen`)
      (`/Engine/EditorBlueprintResources/StandardMacros.DoOnce` false))
    (:`then_1`
      (if (`self.Moving`)
        (`self.MoveWith`)))))

(fn `ClosestPickupPoint`
  (params (Location :type "Vector Structure"))
  (returns (PickupPoint :type "Vector Structure"))
  (locals (ReturnPoint :type "Vector Structure"))
  (bind _returnvalue (`SceneComponent.K2_GetComponentLocation` (`self.Sphere`)))
  (bind _returnvalue_2 (`SceneComponent.K2_GetComponentLocation` (`self.Sphere1`)))
  (if (< (`KismetMathLibrary.Vector_Distance` Location _returnvalue_2) (`KismetMathLibrary.Vector_Distance` Location _returnvalue))
    (bind _output_get (set `local.ReturnPoint` _returnvalue_2))
    (else
      (set `local.ReturnPoint` _returnvalue)))
  (return _output_get))

(fn `IsFull`
  (returns (NewParam :type Boolean))
  (return (== (`self.NumOfProducts`) 24)))

(fn `MoveWith`
  (bind _jackpawn (`self.JackPawn`))
  (bind (_returnvalue_roll _returnvalue_pitch _returnvalue_yaw) (`KismetMathLibrary.BreakRotator` (`self.K2_GetActorRotation` _jackpawn)))
  (if (`self.Moving`)
    (bind _handle (`/Game/Core/RobotJack/BP_RobotJack.GetHandle` _jackpawn))
    (`self.K2_SetActorLocationAndRotation` _handle (`KismetMathLibrary.MakeRotator` _returnvalue_roll _returnvalue_pitch (+ _returnvalue_yaw 90.0)))))

(fn `Resize Widget to Screen`
  (bind _returnvalue (`KismetMathLibrary.MapRangeClamped` (`KismetMathLibrary.VSize` (- (`self.K2_GetActorLocation` (`Controller.K2_GetPawn` (`self.Player Con`))) (`self.K2_GetActorLocation`))) 0.0 3000.0 0.5))
  (`Widget.SetRenderScale` (`self.As Pallet Placement HUD`) (`KismetMathLibrary.MakeVector2D` _returnvalue _returnvalue)))

(fn `UserConstructionScript`)