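; BP_PalletPlacement is a clickable floor spot where the player can place a pallet being moved.
; Tick polls the player controller's MovingPallet flag to switch idle and allowed materials, with a DoOnce preserving the hover highlight.
; Clicking during a move resets the widget and moves the clicked pallet to this actor's XY and rotation at fixed height.
; ClosestDropoffPoint returns whichever of two sphere positions is nearer a given location.
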(event `self.ReceiveBeginPlay`
  (bind _asbp_robotics_fcplayer_controller (cast `/Game/TopDownCPP/Blueprints/BP_RoboticsFCPlayerController` (`GameplayStatics.GetPlayerController` 0)))
  (set `self.PlayerCon` _asbp_robotics_fcplayer_controller))

(event `self.ReceiveTick`
  (params (DeltaSeconds :type "Float (single-precision)"))
  (`self.MaterialForPlacementArea` (`/Game/TopDownCPP/Blueprints/BP_RoboticsFCPlayerController.MovingPallet` (`self.PlayerCon`))))

(event `self.StaticMesh.OnBeginCursorOver`
  (params (TouchedComponent :type "PrimitiveComponent Object Reference"))
  (if (`/Game/TopDownCPP/Blueprints/BP_RoboticsFCPlayerController.MovingPallet` (`self.PlayerCon`))
    (`PrimitiveComponent.SetMaterial` (`self.StaticMesh`) 0 "/Game/Core/Pallet/MI_PalletPlacement_Hover.MI_PalletPlacement_Hover")))

(event `self.StaticMesh.OnEndCursorOver`
  (params (TouchedComponent :type "PrimitiveComponent Object Reference"))
  (if (`/Game/TopDownCPP/Blueprints/BP_RoboticsFCPlayerController.MovingPallet` (`self.PlayerCon`))
    (`PrimitiveComponent.SetMaterial` (`self.StaticMesh`) 0 "/Game/Core/Pallet/MI_PalletPlacement_Allowed.MI_PalletPlacement_Allowed")))

(event `self.StaticMesh.OnClicked`
  (params (TouchedComponent :type "PrimitiveComponent Object Reference") (ButtonPressed :type "Key Structure"))
  (bind (_returnvalue_x _returnvalue_y) (`KismetMathLibrary.BreakVector` (`self.K2_GetActorLocation`)))
  (bind _playercon (`self.PlayerCon`))
  (if (`/Game/TopDownCPP/Blueprints/BP_RoboticsFCPlayerController.MovingPallet` _playercon)
    (`/Game/TopDownCPP/Blueprints/BP_RoboticsFCPlayerController.ResetWidget` _playercon)
    (`Pallet.MovePallet` (`/Game/TopDownCPP/Blueprints/BP_RoboticsFCPlayerController.ClickedPallet` _playercon) (`KismetMathLibrary.MakeVector` _returnvalue_x _returnvalue_y 6.0) (`self.K2_GetActorRotation`))))

(fn `ClosestDropoffPoint`
  (params (Location :type "Vector Structure"))
  (returns (DropoffPoint :type "Vector Structure"))
  (locals (ReturnPoint :type "Vector Structure"))
  (bind _returnvalue (`SceneComponent.K2_GetComponentLocation` (`self.Sphere`)))
  (bind _returnvalue_2 (`SceneComponent.K2_GetComponentLocation` (`self.Sphere1`)))
  (if (< (`KismetMathLibrary.Vector_Distance` Location _returnvalue_2) (`KismetMathLibrary.Vector_Distance` Location _returnvalue))
    (set `local.ReturnPoint` _returnvalue_2)
    (else
      (bind _output_get (set `local.ReturnPoint` _returnvalue))))
  (return _output_get))

(fn `MaterialForPlacementArea`
  (params (Condition :type Boolean))
  (bind _staticmesh (`self.StaticMesh`))
  (if Condition
    (`/Engine/EditorBlueprintResources/StandardMacros.DoOnce` false :!label _label
      (:`Completed`
        (`PrimitiveComponent.SetMaterial` _staticmesh 0 "/Game/Core/Pallet/MI_PalletPlacement_Allowed.MI_PalletPlacement_Allowed")))
    (else
      (`PrimitiveComponent.SetMaterial` _staticmesh 0 "/Game/Core/Pallet/M_PalletPlacement.M_PalletPlacement")
      (goto _label :!via `Reset`))))

(fn `UserConstructionScript`)